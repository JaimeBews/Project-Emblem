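; BP_PlayerController is a player controller that reports the grid index of a clicked tile as a debug message.
; On left click, it traces under the cursor on the Visibility channel and checks that the hit actor's class exactly equals BaseTile.
; It derives the X and Y index by flooring the impact point divided by TileLength, then prints it, with no other gameplay logic.
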(event `Key|LeftMouseButton`
  (params (Key :type "Key Structure"))
  (bind _tile_length (`self.tile length`))
  (bind (_bblockinghit _binitialoverlap _time _distance _location _impactpoint _normal _impactnormal _physmat _hitactor) (`GameplayStatics.BreakHitResult` (`self.GetHitResultUnderCursorByChannel` "TraceTypeQuery1")))
  (:`Pressed`
    (if (== (`GameplayStatics.GetObjectClass` _hitactor) "/Script/ProjectEmblem.BaseTile")
      (`KismetSystemLibrary.PrintString` (`KismetStringLibrary.Concat_StrStr` "This tile is at index[" (`KismetStringLibrary.Conv_IntToString` (`KismetMathLibrary.FFloor` (/ (.x _impactpoint) _tile_length))) "," (`KismetStringLibrary.Conv_IntToString` (`KismetMathLibrary.FFloor` (/ (.y _impactpoint) _tile_length))) "]")))))

(fn `UserConstructionScript`)